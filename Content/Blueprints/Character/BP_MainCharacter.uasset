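; BP_MainCharacter is the main character Blueprint, providing the main HUD widget and camera-based interaction with objects in the world.
; On BeginPlay it creates Widget_Main and adds it to the viewport.
; When IA_Interact starts, it line traces on the Visibility channel from FollowCamera along its forward vector.
; A hit calls InteractMessage on the hit actor, leaving the response to that actor.
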(event `self.ReceiveBeginPlay`
  (bind _returnvalue (`|CreateWidget` "/Game/Blueprints/Widgets/Widget_Main.Widget_Main_C"))
  (`UserWidget.AddToViewport` _returnvalue 0))

(event `EnhancedInput|/Game/ThirdPerson/Input/Actions/IA_Interact`
  (params (ActionValue :type Boolean) (ElapsedSeconds :type "Float (double-precision)") (TriggeredSeconds :type "Float (double-precision)") (InputAction :type "InputAction Object Reference" :default "/Game/ThirdPerson/Input/Actions/IA_Interact.IA_Interact"))
  (bind _followcamera (`self.FollowCamera`))
  (bind _returnvalue (`SceneComponent.K2_GetComponentLocation` _followcamera))
  (:`Started`
    (bind (_outhit _returnvalue_2) (`KismetSystemLibrary.LineTraceSingle` _returnvalue (+ _returnvalue (* (`SceneComponent.GetForwardVector` _followcamera) 800.0)) "TraceTypeQuery1"))
    (if _returnvalue_2
      (message `/Game/Blueprints/BPI/BPI_Interact.Interact` (`.HitActor` (`GameplayStatics.BreakHitResult` _outhit))))))

(fn `UserConstructionScript`)