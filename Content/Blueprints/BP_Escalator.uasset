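; BP_Escalator is an escalator that builds a diagonal run of static-mesh steps and moves them in an endless loop.
; The construction script spawns steps from NumofStairs, randomly choosing between two mesh-component nodes, then rotates them.
; Tick nudges each root child by a fixed world offset, independent of frame time.
; A box overlap with BP_BoxCollision sends that step back to the root's location.
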(event `self.ReceiveBeginPlay`)

(event `self.ReceiveTick`
  (params (DeltaSeconds :type "Float (single-precision)"))
  (for _array_element (`SceneComponent.GetChildrenComponents` (`self.DefaultSceneRoot`) false)
    (`SceneComponent.K2_AddWorldOffset` _array_element (1.0 0.0 1.0) false false)
    (bind (_outactors _returnvalue) (`KismetSystemLibrary.BoxOverlapActors` (`SceneComponent.K2_GetComponentLocation` _array_element) (15.0 15.0 15.0) (`|MakeArray` "ObjectTypeQuery2" :!type "EObjectTypeQuery Enum") "/Game/Blueprints/BP_BoxCollision.BP_BoxCollision_C"))
    (if _returnvalue
      (`SceneComponent.K2_SetWorldLocation` _array_element (`SceneComponent.K2_GetComponentLocation` (`self.DefaultSceneRoot`)) false false))))

(fn `UserConstructionScript`
  (for _index (range (+ (`self.NumofStairs`) 1))
    (if (> (`KismetMathLibrary.RandomFloat`) 0.7)
      (`AddComponent|NODE_AddStaticMeshComponent-0` :`RelativeTransform` (`KismetMathLibrary.MakeTransform` (`KismetMathLibrary.MakeVector` 0.0 (`KismetMathLibrary.Conv_IntToDouble` (* _index -30)) (`KismetMathLibrary.Conv_IntToDouble` (* _index 30)))))
      (else
        (`AddComponent|NODE_AddStaticMeshComponent-1` :`RelativeTransform` (`KismetMathLibrary.MakeTransform` (`KismetMathLibrary.MakeVector` 0.0 (`KismetMathLibrary.Conv_IntToDouble` (* _index -30)) (`KismetMathLibrary.Conv_IntToDouble` (* _index 30))))))))
  (for _array_element (`SceneComponent.GetChildrenComponents` (`self.DefaultSceneRoot`) false)
    (`SceneComponent.K2_SetRelativeRotation` _array_element (struct :`Pitch` -90.0) false false)))